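; BP_ComboBase manages item combinations defined in the DataCombo data table and looks up the combo for a given pair of items.
; PopulateCache reads every row and builds a nested map cache, storing each pair in both orders so lookup is order-independent.
; GetCombo resolves two items to a row name through the cache, then returns that table row with a found flag.
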(fn `GetCombo`
  (params (Item1 :type "/Game/Items/DA_Item Object Reference") (Item2 :type "/Game/Items/DA_Item Object Reference"))
  (returns (Found :type Boolean) (Combo :type "/Game/Items/S_Combo Structure"))
  (bind (_value _returnvalue) (`BlueprintMapLibrary.Map_Find` (`self.Cache`) Item1))
  (if _returnvalue
    (bind (_value_2 _returnvalue_2) (`BlueprintMapLibrary.Map_Find` (break `/Game/Items/S_CacheEntry` _value) Item2))
    (if _returnvalue_2
      (bind _returnvalue_3 (`|GetDataTableRow` (`self.DataCombo`) _value_2)
        (:`then`
          (return true _returnvalue_3))
        (:`RowNotFound`
          _))))
  (return false))

(fn `PopulateCache`
  (bind _datacombo (`self.DataCombo`))
  ; Constitue le cache
  (`BlueprintMapLibrary.Map_Clear` (`self.Cache`))
  (bind _outrownames (`DataTableFunctionLibrary.GetDataTableRowNames` _datacombo))
  (for _array_element _outrownames
    (bind _returnvalue (`|GetDataTableRow` _datacombo _array_element)
      (:`then`
        (bind (_item _item2) (break `/Game/Items/S_Combo` _returnvalue))
        ;; Cree tableau double entree :
        ;; Cache[Ring][Potion]
        ;; Cache[Potion][Ring]
        (`self.PopulateCacheEntry` _item _item2 _array_element)
        (`self.PopulateCacheEntry` _item2 _item _array_element)))))

(fn `PopulateCacheEntry`
  (params (Item1 :type "/Game/Items/DA_Item Object Reference") (Item2 :type "/Game/Items/DA_Item Object Reference") (NameCombo :type Name))
  (locals (CacheEntry :type "Map of /Game/Items/DA_Item Object Reference to Name"))
  (bind _cacheentry (`local.CacheEntry`))
  (bind (_value _returnvalue) (`BlueprintMapLibrary.Map_Find` (`self.Cache`) Item1))
  (if _returnvalue
    (set `local.CacheEntry` (break `/Game/Items/S_CacheEntry` _value))
    (else
      (set `local.CacheEntry` (`|MakeMap`))))
  (`BlueprintMapLibrary.Map_Add` _cacheentry Item2 NameCombo)
  (`BlueprintMapLibrary.Map_Add` (`self.Cache`) Item1 (make `/Game/Items/S_CacheEntry` _cacheentry)))
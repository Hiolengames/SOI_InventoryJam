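; BP_SwitchNextPhase is an interactable actor that moves a two-player game to its next phase once both players have readied up.
; Interact records the interacting player index as ready, prints a message and freezes that character by setting its movement mode to None.
; When both flags are set, it switches each top-down character to its inventory phase and calls SwitchPhases on BP_TopDownGameMode.
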(event `/Game/Items/I_Interact.Interact`
  (params (`Index Player` :type Integer))
  (if (== `Index Player` 0)
    (set `self.hasP1interacted` true)
    (`KismetSystemLibrary.PrintString` "P1 ready")
    (`CharacterMovementComponent.SetMovementMode` (`Character.CharacterMovement` (`GameplayStatics.GetPlayerCharacter` 0)) "MOVE_None" 0)
    (`self.ArePlayersReady`)
    (elif (== `Index Player` 1)
      (set `self.hasP2interacted` true)
      (`KismetSystemLibrary.PrintString` "P2 ready")
      (`CharacterMovementComponent.SetMovementMode` (`Character.CharacterMovement` (`GameplayStatics.GetPlayerCharacter` 1)) "MOVE_None" 0)
      (`self.ArePlayersReady`))))

(event `ArePlayersReady`
  (if (and (`self.hasP2interacted`) (`self.hasP1interacted`))
    (bind _asbp_top_down_character (cast `/Game/TopDown/Blueprints/BP_TopDownCharacter` (`GameplayStatics.GetPlayerCharacter` 0)))
    (`/Game/TopDown/Blueprints/BP_TopDownCharacter.SwitchToInventoryPhase` _asbp_top_down_character)
    (bind _asbp_top_down_character_2 (cast `/Game/TopDown/Blueprints/BP_TopDownCharacter2` (`GameplayStatics.GetPlayerCharacter` 1)))
    (`/Game/TopDown/Blueprints/BP_TopDownCharacter2.SwitchToInventoryPhaseP2` _asbp_top_down_character_2)
    (bind _asbp_top_down_game_mode (cast `/Game/TopDown/Blueprints/BP_TopDownGameMode` (`GameplayStatics.GetGameMode`)))
    (`/Game/TopDown/Blueprints/BP_TopDownGameMode.SwitchPhases` _asbp_top_down_game_mode)))

(fn `UserConstructionScript`)
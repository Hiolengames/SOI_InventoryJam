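; BP_SpawnArea is an actor that scatters items from a list inside a box area over time.
; On BeginPlay it copies the item list and starts a looping timer.
; Each tick spawns a BPA_BaseItem with random item data at a random XY point in the box and fixed height, adjusting for collisions or skipping the spawn.
; It removes the picked entry, stopping the timer when the list is empty.
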(event `self.ReceiveBeginPlay`
  (set `self.LocalItemsList` (`/Game/Items/DA_ItemList.Items` (`self.ItemsList`)))
  (`self.StartSpawnItems`))

(event `StopSpawnItems`
  (`KismetSystemLibrary.K2_ClearAndInvalidateTimerHandle` (stale `StartSpawnItems` _returnvalue)))

(event `StartSpawnItems`
  (if (`KismetArrayLibrary.Array_IsNotEmpty` (`self.LocalItemsList`))
    (bind _returnvalue (`KismetSystemLibrary.K2_SetTimerDelegate` (delegate `SpawnItemsOvertime`) 1.5 true))))

(event `SpawnItemsOvertime`
  (bind _spawnarea (`self.SpawnArea`))
  (bind _localitemslist (`self.LocalItemsList`))
  (bind (_returnvalue_x _returnvalue_y) (`KismetMathLibrary.BreakVector` (`KismetMathLibrary.RandomPointInBoundingBox` (`SceneComponent.K2_GetComponentLocation` _spawnarea) (`BoxComponent.BoxExtent` _spawnarea))))
  (bind (_outitem _outindex) (`KismetArrayLibrary.Array_Random` (`self.LocalItemsList`)))
  (`|SpawnActorFromClass` "/Game/Items/BPA_BaseItem.BPA_BaseItem_C" (`KismetMathLibrary.MakeTransform` (`KismetMathLibrary.MakeVector` _returnvalue_x _returnvalue_y 15.0)) "AdjustIfPossibleButDontSpawnIfColliding" "MultiplyWithRoot" null (`/Game/Items/DA_Item.Data` _outitem) null)
  (`KismetArrayLibrary.Array_Remove` _localitemslist _outindex)
  (if (`KismetArrayLibrary.Array_IsEmpty` _localitemslist)
    (`self.StopSpawnItems`)))

(fn `UserConstructionScript`)
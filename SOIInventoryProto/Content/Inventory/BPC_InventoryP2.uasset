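; Inventory component for the second player, which builds and drives that player's inventory widget on screen.
; On BeginPlay it creates WB_Inventory2 for player controller 1 and sizes the item array from the widget's slot children.
; Added items fill the first empty slot, and a refresh paints each slot with the item flipbook's first sprite or a translucent placeholder.
; Switching to inventory gives that widget UI-only input and keyboard focus.
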(event `self.ReceiveBeginPlay`
  (bind _returnvalue (`|CreateWidget` "/Game/Inventory/WB_Inventory2.WB_Inventory2_C" (`GameplayStatics.GetPlayerController` 1)))
  (bind _output_get (set `self.InventoryP2` _returnvalue))
  (`self.InitializeInventory`)
  (`self.RefreshInventory`)
  (`UserWidget.AddToViewport` _output_get 0))

(fn `AddToInventory`
  (params (ItemToAdd :type "/Game/Items/S_Item Structure"))
  (returns (ItemAdded :type Boolean))
  (locals (Item :type "/Game/Items/S_Item Structure"))
  (set `local.Item` ItemToAdd)
  (for (_array_element _array_index) (`self.Items`)
    (if (`KismetStringLibrary.IsEmpty` (break `/Game/Items/S_Item` _array_element))
      (`KismetArrayLibrary.Array_Set` (`self.Items`) _array_index (`local.Item`))
      (`self.RefreshInventory`)
      (return true)))
  (return false))

(fn `InitializeInventory`
  (for _ (`PanelWidget.GetAllChildren` (`/Game/Inventory/WB_Inventory2.Slots` (`self.InventoryP2`)))
    (`KismetArrayLibrary.Array_Add` (`self.Items`) (make `/Game/Items/S_Item` "" null))))

(fn `RefreshInventory`
  (locals (Slot :type "/Game/Inventory/WB_InventorySlot Object Reference"))
  (for (_array_element _array_index) (`self.Items`)
    (bind _aswb_inventory_slot (cast `/Game/Inventory/WB_InventorySlot` (`PanelWidget.GetChildAt` (`/Game/Inventory/WB_Inventory2.Slots` (`self.InventoryP2`)) _array_index)))
    (set `local.Slot` _aswb_inventory_slot)
    (if (`KismetStringLibrary.IsEmpty` (break `/Game/Items/S_Item` _array_element))
      (`Image.SetBrush` (`/Game/Inventory/WB_InventorySlot.Item` (`local.Slot`)) (`WidgetBlueprintLibrary.MakeBrushFromMaterial` "/Paper2D/TranslucentUnlitSpriteMaterial.TranslucentUnlitSpriteMaterial"))
      (else
        (`Image.SetBrush` (`/Game/Inventory/WB_InventorySlot.Item` (`local.Slot`)) (`PaperSpriteBlueprintLibrary.MakeBrushFromSprite` (`PaperFlipbook.GetSpriteAtFrame` (`.Flipbook_5_A146A23E473FD3D9ED6181ABF298AADB` (break `/Game/Items/S_Item` _array_element)) 0)))))))

(fn `SwitchToInventory`
  (bind _inventoryp2 (`self.InventoryP2`))
  (`WidgetBlueprintLibrary.SetInputMode_UIOnlyEx` (`GameplayStatics.GetPlayerController` 1) _inventoryp2)
  (`Widget.SetKeyboardFocus` _inventoryp2)
  (`/Game/Inventory/WB_Inventory2.SwitchInventoryFormatP2` _inventoryp2))
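; Inventory component that stores a player's item data assets and displays them in a WB_Inventory widget, with support for two players.
; Items fill the first empty slot, with DA_Empty marking free ones; refreshes draw flipbook first frames into slot widgets.
; A focus flag selects between Collect and Inventory slot layouts.
; Combo validation pairs an item with one from the second player's inventory through the game instance's ComboBase.
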(fn `AddToInventory`
  (params (ItemToAdd :type "/Game/Items/DA_Item Object Reference"))
  (returns (ItemAdded :type Boolean))
  (locals (Item :type "/Game/Items/S_Item Structure") (Daitem :type "/Game/Items/DA_Item Object Reference"))
  (set `local.Daitem` ItemToAdd)
  ; Check If there is a spot left in the inventory to add the item the player overlapped
  (for (_array_element _array_index) (`self.Items`)
    (bind _data_name (break `/Game/Items/S_Item` (`/Game/Items/DA_Item.Data` _array_element)))
    (if (`KismetStringLibrary.IsEmpty` _data_name)
      (`KismetArrayLibrary.Array_Set` (`self.Items`) _array_index (`local.Daitem`))
      (`self.RefreshInventory`)
      (return true)))
  (return false))

(fn `CreateInventory`
  (params (PlayerController :type "PlayerController Object Reference"))
  ; Create Inventory Widget and initialize it
  (bind _returnvalue (`|CreateWidget` "/Game/Inventory/WB_Inventory.WB_Inventory_C" PlayerController (`self.IsPlayer2`)))
  (set `self.Inventory` _returnvalue)
  (`self.InitializeInventory`)
  (`self.RefreshInventory`)
  (`UserWidget.AddToViewport` _returnvalue 0)
  (`EnhancedInputSubsystemInterface.RemoveMappingContext` (pcsubsystem `EnhancedInputLocalPlayerSubsystem` (`GameplayStatics.GetPlayerController` 0)) "/Game/Input/IMC_Inventory.IMC_Inventory" (struct)))

(fn `DeleteFromInventory`
  (params (IndexItemToDelete :type Integer))
  (`KismetArrayLibrary.Array_Set` (`self.Items`) IndexItemToDelete "/Game/Items/ItemsData/DA_Empty.DA_Empty"))

(fn `InitializeInventory`
  (for _ (`PanelWidget.GetAllChildren` (`/Game/Inventory/WB_Inventory.Slots` (`self.Inventory`)))
    (`KismetArrayLibrary.Array_Add` (`self.Items`) "/Game/Items/ItemsData/DA_Empty.DA_Empty")))

(fn `IsComboValid`
  (params (IndexItemP1 :type Integer) (IndexItemP2 :type Integer))
  (returns (CanCombo :type Boolean) (ComboValue :type Integer))
  (bind _output (`|GetArrayItem` (`self.Items`) IndexItemP1))
  (bind _asbp_top_down_character (cast `/Game/TopDown/Blueprints/BP_TopDownCharacter` (`GameplayStatics.GetPlayerCharacter` 1)))
  (`KismetSystemLibrary.PrintString` (`KismetStringLibrary.Concat_StrStr` "Item 1 DA Item name : " (`KismetSystemLibrary.GetDisplayName` _output)))
  (bind _output_2 (`|GetArrayItem` (`/Game/Inventory/BPC_Inventory.Items` (`/Game/TopDown/Blueprints/BP_TopDownCharacter.BPC_Inventory` _asbp_top_down_character)) IndexItemP2))
  (`KismetSystemLibrary.PrintString` (`KismetStringLibrary.Concat_StrStr` "Item 2 DA Item name : " (`KismetSystemLibrary.GetDisplayName` _output_2)))
  (bind _asbp_top_down_game_instance (cast `/Game/TopDown/Blueprints/BP_TopDownGameInstance` (`GameplayStatics.GetGameInstance`)))
  (bind (_found _combo) (`/Game/Items/BP_ComboBase.GetCombo` (`/Game/TopDown/Blueprints/BP_TopDownGameInstance.ComboBase` _asbp_top_down_game_instance) _output _output_2))
  (return _found (`.Value_5_8C1DFE30467317590BD56080CBEC7127` (break `/Game/Items/S_Combo` _combo))))

(fn `RefreshInventory`
  (locals (Slot :type "/Game/Inventory/WB_InventorySlot Object Reference") (SlotI :type "/Game/Inventory/WB_InventorySlot Object Reference"))
  (for (_array_element _array_index) (`self.Items`)
    (if (`self.isInventoryFocus`)
      ; If player is in phase "Collect"
      (bind _aswb_inventory_slot (cast `/Game/Inventory/WB_InventorySlot` (`PanelWidget.GetChildAt` (`/Game/Inventory/WB_Inventory.SlotsInventory` (`self.Inventory`)) _array_index)))
      (set `local.SlotI` _aswb_inventory_slot)
      (bind (_name _flipbook) (break `/Game/Items/S_Item` (`/Game/Items/DA_Item.Data` _array_element)))
      (if (`KismetStringLibrary.IsEmpty` _name)
        (`Image.SetBrush` (`/Game/Inventory/WB_InventorySlot.Item` (`local.SlotI`)) (`WidgetBlueprintLibrary.MakeBrushFromMaterial` "/Paper2D/TranslucentUnlitSpriteMaterial.TranslucentUnlitSpriteMaterial"))
        (else
          (`Image.SetBrush` (`/Game/Inventory/WB_InventorySlot.Item` (`local.SlotI`)) (`PaperSpriteBlueprintLibrary.MakeBrushFromSprite` (`PaperFlipbook.GetSpriteAtFrame` _flipbook 0)))))
      (else
        ; If player is in phase "Inventory"
        (bind _aswb_inventory_slot_2 (cast `/Game/Inventory/WB_InventorySlot` (`PanelWidget.GetChildAt` (`/Game/Inventory/WB_Inventory.Slots` (`self.Inventory`)) _array_index)))
        (set `local.Slot` _aswb_inventory_slot_2)
        (if (`KismetStringLibrary.IsEmpty` _name)
          ;; If slot is empty, reset item image
          (`Image.SetBrush` (`/Game/Inventory/WB_InventorySlot.Item` (`local.Slot`)) (`WidgetBlueprintLibrary.MakeBrushFromMaterial` "/Paper2D/TranslucentUnlitSpriteMaterial.TranslucentUnlitSpriteMaterial"))
          (else
            ;; There is an object in the slot, so show the proper element image
            (`Image.SetBrush` (`/Game/Inventory/WB_InventorySlot.Item` (`local.Slot`)) (`PaperSpriteBlueprintLibrary.MakeBrushFromSprite` (`PaperFlipbook.GetSpriteAtFrame` _flipbook 0)))))))))

(fn `SwitchToCollect`
  (set `self.isInventoryFocus` false)
  (`self.RefreshInventory`))

(fn `SwitchToInventory`
  (bind _inventory (`self.Inventory`))
  (if (not (`self.IsPlayer2`))
    (`WidgetBlueprintLibrary.SetInputMode_GameAndUIEx` (`GameplayStatics.GetPlayerController` 0) _inventory))
  (`/Game/Inventory/WB_Inventory.SwitchInventoryFormat` _inventory)
  (set `self.isInventoryFocus` true)
  (`self.RefreshInventory`))